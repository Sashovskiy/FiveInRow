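; Game mode Blueprint that runs the match flow from main menu through game start to win screen.
; BeginPlay shows the MainMenu widget and binds SWiinEvent to the win notification, which replaces all widgets with a WinScreen showing the winner.
; StartGame calls Start, then centers the player pawn and scales the TestPawn spring arm from GetSize, using a 110-unit spacing.
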(event `self.ReceiveBeginPlay`
  (bind _returnvalue (`|CreateWidget` "/Game/MainMenu.MainMenu_C"))
  (`UserWidget.AddToViewport` _returnvalue 0)
  (add `self.SomeOneWin` (delegate `SWiinEvent`)))

(event `SWiinEvent`
  (`WidgetLayoutLibrary.RemoveAllWidgets`)
  (bind _returnvalue (`|CreateWidget` "/Game/WinScreen.WinScreen_C" null (`self.GetWinner`)))
  (`UserWidget.AddToViewport` _returnvalue 0))

(event `StartGame`
  (bind _returnvalue (`self.GetSize`))
  (bind _returnvalue_2 (`GameplayStatics.GetPlayerPawn` 0))
  (bind _returnvalue_3 (- (* (/ (`KismetMathLibrary.Conv_IntToDouble` _returnvalue) 2.0) 110.0) (/ 110.0 2.0)))
  (`self.Start`)
  (`self.K2_SetActorLocation` _returnvalue_2 (`KismetMathLibrary.MakeVector` _returnvalue_3 _returnvalue_3 112.0) false false)
  (bind _astest_pawn (cast `/Game/TestPawn` _returnvalue_2))
  (set `SpringArmComponent.TargetArmLength` (* _returnvalue 110.0) (`/Game/TestPawn.SpringArm` _astest_pawn)))

(fn `UserConstructionScript`)